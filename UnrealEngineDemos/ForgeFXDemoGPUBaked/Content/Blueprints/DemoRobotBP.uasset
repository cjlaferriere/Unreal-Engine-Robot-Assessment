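; Demo robot Blueprint with a draggable toy robot and detachable right arm, an orbit camera, and main, demo and pause menus.
; Clicking torso or arm starts a Delay-looped cursor line trace that moves the part in world X/Y.
; The arm attaches or detaches by snap distance, updating highlight materials and status UI.
; Gated, self-retriggering timers drive held-key orbit, pitch and zoom, alongside angle snaps and reset.
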(event `LoopRobotDrag`
  (bind (_worldlocation _worlddirection) (`PlayerController.DeprojectMousePositionToWorld` (`GameplayStatics.GetPlayerController` 0)))
  ; Robot Torso Logic
  ;; Drag Robot Via Line Trace
  (bind _outhit (`KismetSystemLibrary.LineTraceSingle` :`Start` _worldlocation :`End` (+ _worldlocation (* _worlddirection 10000.0)) :`TraceChannel` "TraceTypeQuery3" :`bIgnoreSelf` false))
  (`SceneComponent.K2_SetWorldLocation` (`self.Robot`) (`KismetMathLibrary.MakeVector` (.x (`.Location` (`GameplayStatics.BreakHitResult` _outhit))) (.y (`.Location` (`GameplayStatics.BreakHitResult` _outhit)))) false false)
  (`KismetSystemLibrary.Delay` 0.05)
  (if (`self.IsDraggingRobot`)
    (`self.LoopRobotDrag`)))

(event `InputAction|Interact`
  (params (Key :type "Key Structure"))
  ; Action Inputs
  ;; Interact, Ensure Limb Is Reset To Robot Material
  (:`Released`
    (`|ExecutionSequence`
      (:`then_0`
        (set `self.IsDraggingRobot` false))
      (:`then_1`
        (set `self.IsDraggingLimb` false)
        (`PrimitiveComponent.SetMaterial` (`self.RightUpperArmOBJ`) 0 "/Game/Materials/RobotToy/RobotToyMaterial.RobotToyMaterial")
        (`PrimitiveComponent.SetMaterial` (`self.RightLowerArmOBJ`) 0 "/Game/Materials/RobotToy/RobotToyMaterial.RobotToyMaterial")
        (`PrimitiveComponent.SetMaterial` (`self.RightHandOBJ`) 0 "/Game/Materials/RobotToy/RobotToyMaterial.RobotToyMaterial")))))

(event `self.ReceiveBeginPlay`
  ; Initialization
  ;; Initialize UI & Mouse
  (`|ExecutionSequence`
    (:`then_0`
      (bind _returnvalue (`|GenericCreateObject` "/Game/UI/MainMenuUI.MainMenuUI_C"))
      (bind _output_get (set `self.MainMenuUIWidget` _returnvalue))
      (`UserWidget.AddToViewport` _output_get 0)
      (`WidgetBlueprintLibrary.SetInputMode_GameAndUIEx` (`GameplayStatics.GetPlayerController` 0) (`self.MainMenuUIWidget`) "DoNotLock" false))
    (:`then_1`
      (bind _returnvalue_2 (`|CreateWidget` "/Game/UI/DemoUI.DemoUI_C" (`GameplayStatics.GetPlayerController` 0)))
      (set `self.DemoUIWidget` _returnvalue_2))
    (:`then_2`
      (bind _returnvalue_3 (`|GenericCreateObject` "/Game/UI/PauseMenuHUD.PauseMenuHUD_C"))
      (set `self.PauseMenuUIWidget` _returnvalue_3))
    (:`then_3`
      (set `PlayerController.bShowMouseCursor` true (`GameplayStatics.GetPlayerController` 0)))))

(event `CameraUpRetrigger`
  (bind _returnvalue (`GameplayStatics.GetPlayerController` 0))
  (bind _springarm (`self.SpringArm`))
  (bind (_relativerotation_roll _relativerotation_pitch) (`KismetMathLibrary.BreakRotator` (`SceneComponent.RelativeRotation` _springarm)))
  ; Camera Inputs
  ;; Move Camera Up
  (if (not (`self.IsMenuOpen`))
    (`/Engine/EditorBlueprintResources/StandardMacros.Gate` true :!label _label
      (:`Exit`
        (`KismetSystemLibrary.K2_SetTimerDelegate` (delegate `CameraUpRetrigger`) 0.025 :!label _label_2)
        (if (`KismetMathLibrary.BooleanNOR` (`PlayerController.IsInputKeyDown` _returnvalue "S") (`PlayerController.IsInputKeyDown` _returnvalue "Down"))
          (if (<= _relativerotation_pitch -87.5)
            (`SceneComponent.K2_SetRelativeRotation` _springarm (struct :`Pitch` -89.0) false false)
            (else
              (`SceneComponent.K2_AddLocalRotation` _springarm (struct :`Pitch` -1.5) false false))))))))

(event `LoopRightArmDrag`
  (bind (_worldlocation _worlddirection) (`PlayerController.DeprojectMousePositionToWorld` (`GameplayStatics.GetPlayerController` 0)))
  ; Robot Right Arm Logic
  ;; Drag Robot Right Arm Via Line Trace
  (bind _outhit (`KismetSystemLibrary.LineTraceSingle` :`Start` _worldlocation :`End` (+ _worldlocation (* _worlddirection 10000.0)) :`TraceChannel` "TraceTypeQuery3" :`bIgnoreSelf` false))
  (if (<= (`KismetMathLibrary.VSize` (- (`SceneComponent.K2_GetComponentLocation` (`self.Robot`)) (`.Location` (`GameplayStatics.BreakHitResult` _outhit)))) (`self.SnapDistance`))
    (`SceneComponent.K2_AttachToComponent` (`self.RightArm`) (`self.Robot`) "None" "KeepWorld" "KeepWorld" "KeepWorld" true)
    (`SceneComponent.K2_SetRelativeLocation` (`self.RightArm`) (0.0 0.0 0.0) false false)
    (`PrimitiveComponent.SetMaterial` (`self.RightLowerArmOBJ`) 0 "/Game/Shaders/GreenShader.GreenShader")
    (`PrimitiveComponent.SetMaterial` (`self.RightHandOBJ`) 0 "/Game/Shaders/GreenShader.GreenShader")
    (`PrimitiveComponent.SetMaterial` (`self.RightUpperArmOBJ`) 0 "/Game/Shaders/GreenShader.GreenShader")
    (`/Game/UI/DemoUI.PrintStatusATTACHED` (`self.DemoUIWidget`))
    (`KismetSystemLibrary.Delay` 0.05)
    (if (`self.IsDraggingLimb`)
      (`self.LoopRightArmDrag`))
    (else
      (`SceneComponent.K2_DetachFromComponent` (`self.RightArm`) "KeepWorld" "KeepWorld" "KeepWorld" true)
      (`SceneComponent.K2_SetWorldLocation` (`self.RightArm`) (`KismetMathLibrary.MakeVector` (.x (`.Location` (`GameplayStatics.BreakHitResult` _outhit))) (.y (`.Location` (`GameplayStatics.BreakHitResult` _outhit)))) false false)
      (`PrimitiveComponent.SetMaterial` (`self.RightLowerArmOBJ`) 0 "/Game/Shaders/YellowShader.YellowShader")
      (`PrimitiveComponent.SetMaterial` (`self.RightHandOBJ`) 0 "/Game/Shaders/YellowShader.YellowShader")
      (`PrimitiveComponent.SetMaterial` (`self.RightUpperArmOBJ`) 0 "/Game/Shaders/YellowShader.YellowShader")
      (`/Game/UI/DemoUI.PrintStatusDETACHED` (`self.DemoUIWidget`))
      (`KismetSystemLibrary.Delay` 0.05)
      (if (`self.IsDraggingLimb`)
        (`self.LoopRightArmDrag`)))))

(event `InputAction|CameraUp`
  (params (Key :type "Key Structure"))
  ; Camera Inputs
  ;; Move Camera Up
  (:`Pressed`
    (if (not (`self.IsMenuOpen`))
      (`|ExecutionSequence`
        (:`then_0`
          (goto _label :!via `Open`))
        (:`then_1`
          (goto _label_2)))))
  (:`Released`
    (goto _label :!via `Close`)))

(event `self.TorsoOBJ.OnClicked`
  (params (TouchedComponent :type "PrimitiveComponent Object Reference") (ButtonPressed :type "Key Structure"))
  ; Robot Torso Logic
  ;; Torso Clicked, Start Drag
  (set `self.IsDraggingRobot` true)
  (`self.LoopRobotDrag`))

(event `InputAction|Pause`
  (params (Key :type "Key Structure"))
  (bind _returnvalue (`GameplayStatics.GetPlayerController` 0))
  (bind _returnvalue_2 (`GameplayStatics.GetPlayerController` 0))
  ; Action Inputs
  ;; Pause Game
  (:`Pressed`
    (if (not (`self.IsMenuOpen`))
      (set `self.IsMenuOpen` true)
      (set `PlayerController.bEnableClickEvents` false _returnvalue_2)
      (set `PlayerController.bEnableMouseOverEvents` false _returnvalue_2)
      (`GameplayStatics.SetGamePaused` true)
      (`Widget.RemoveFromParent` (`self.DemoUIWidget`))
      (`UserWidget.AddToViewport` (`self.PauseMenuUIWidget`) 0)
      (`WidgetBlueprintLibrary.SetInputMode_UIOnlyEx` _returnvalue (`self.PauseMenuUIWidget`))
      (`EnhancedInputLibrary.FlushPlayerInput` _returnvalue))))

(event `CameraDownRetrigger`
  (bind _returnvalue (`GameplayStatics.GetPlayerController` 0))
  (bind _springarm (`self.SpringArm`))
  (bind (_relativerotation_roll _relativerotation_pitch) (`KismetMathLibrary.BreakRotator` (`SceneComponent.RelativeRotation` _springarm)))
  ; Camera Inputs
  ;; Move Camera Down
  (if (not (`self.IsMenuOpen`))
    (`/Engine/EditorBlueprintResources/StandardMacros.Gate` true :!label _label_3
      (:`Exit`
        (`KismetSystemLibrary.K2_SetTimerDelegate` (delegate `CameraDownRetrigger`) 0.025 :!label _label_4)
        (if (`KismetMathLibrary.BooleanNOR` (`PlayerController.IsInputKeyDown` _returnvalue "W") (`PlayerController.IsInputKeyDown` _returnvalue "Up"))
          (if (>= _relativerotation_pitch 28.5)
            (`SceneComponent.K2_SetRelativeRotation` _springarm (struct :`Pitch` 30.0) false false)
            (else
              (`SceneComponent.K2_AddLocalRotation` _springarm (struct :`Pitch` 1.5) false false))))))))

(event `self.TorsoOBJ.OnBeginCursorOver`
  (params (TouchedComponent :type "PrimitiveComponent Object Reference"))
  ; Robot Torso Logic
  ;; Cursor Over Torso, Set Robot Yellow
  (if (`self.IsDraggingRobot`)
    _
    (elif (not (`self.IsDraggingLimb`))
      (`PrimitiveComponent.SetMaterial` (`self.TorsoOBJ`) 0 "/Game/Shaders/YellowShader.YellowShader")
      (`PrimitiveComponent.SetMaterial` (`self.HipsOBJ`) 0 "/Game/Shaders/YellowShader.YellowShader")
      (`PrimitiveComponent.SetMaterial` (`self.HeadOBJ`) 0 "/Game/Shaders/YellowShader.YellowShader")
      (`PrimitiveComponent.SetMaterial` (`self.JawOBJ`) 0 "/Game/Shaders/YellowShader.YellowShader")
      (`PrimitiveComponent.SetMaterial` (`self.LeftEyeOBJ`) 0 "/Game/Shaders/YellowShader.YellowShader")
      (`PrimitiveComponent.SetMaterial` (`self.RightEyeOBJ`) 0 "/Game/Shaders/YellowShader.YellowShader")
      (`PrimitiveComponent.SetMaterial` (`self.NeckOBJ`) 0 "/Game/Shaders/YellowShader.YellowShader")
      (`PrimitiveComponent.SetMaterial` (`self.RightUpperArmOBJ`) 0 "/Game/Shaders/YellowShader.YellowShader")
      (`PrimitiveComponent.SetMaterial` (`self.RightLowerArmOBJ`) 0 "/Game/Shaders/YellowShader.YellowShader")
      (`PrimitiveComponent.SetMaterial` (`self.RightHandOBJ`) 0 "/Game/Shaders/YellowShader.YellowShader")
      (`PrimitiveComponent.SetMaterial` (`self.LeftUpperArmOBJ`) 0 "/Game/Shaders/YellowShader.YellowShader")
      (`PrimitiveComponent.SetMaterial` (`self.LeftLowerArmOBJ`) 0 "/Game/Shaders/YellowShader.YellowShader")
      (`PrimitiveComponent.SetMaterial` (`self.LeftHandOBJ`) 0 "/Game/Shaders/YellowShader.YellowShader")
      (`PrimitiveComponent.SetMaterial` (`self.RightThighOBJ`) 0 "/Game/Shaders/YellowShader.YellowShader")
      (`PrimitiveComponent.SetMaterial` (`self.RightShinOBJ`) 0 "/Game/Shaders/YellowShader.YellowShader")
      (`PrimitiveComponent.SetMaterial` (`self.RightFootOBJ`) 0 "/Game/Shaders/YellowShader.YellowShader")
      (`PrimitiveComponent.SetMaterial` (`self.LeftThighOBJ`) 0 "/Game/Shaders/YellowShader.YellowShader")
      (`PrimitiveComponent.SetMaterial` (`self.LeftShinOBJ`) 0 "/Game/Shaders/YellowShader.YellowShader")
      (`PrimitiveComponent.SetMaterial` (`self.LeftFootOBJ`) 0 "/Game/Shaders/YellowShader.YellowShader"))))

(event `InputAction|CameraDown`
  (params (Key :type "Key Structure"))
  ; Camera Inputs
  ;; Move Camera Down
  (:`Pressed`
    (if (not (`self.IsMenuOpen`))
      (`|ExecutionSequence`
        (:`then_0`
          (goto _label_3 :!via `Open`))
        (:`then_1`
          (goto _label_4)))))
  (:`Released`
    (goto _label_3 :!via `Close`)))

(event `StartDemo`
  (bind _returnvalue (`GameplayStatics.GetPlayerController` 0))
  (bind _demouiwidget (`self.DemoUIWidget`))
  ; Initialization
  ;; Start Demo
  (`|ExecutionSequence`
    (:`then_0`
      (`Widget.RemoveFromParent` (`self.MainMenuUIWidget`))
      (`UserWidget.AddToViewport` _demouiwidget 0)
      (`WidgetBlueprintLibrary.SetInputMode_GameAndUIEx` _returnvalue _demouiwidget "DoNotLock" false)
      (`WidgetBlueprintLibrary.SetFocusToGameViewport`)
      (set `PlayerController.bEnableClickEvents` true _returnvalue)
      (set `PlayerController.bEnableMouseOverEvents` true _returnvalue))
    (:`then_1`
      (`EnhancedInputLibrary.FlushPlayerInput` (`GameplayStatics.GetPlayerController` 0))
      (set `self.IsMenuOpen` false)
      (set `self.CanPause` true))))

(event `self.RightUpperArmOBJ.OnClicked`
  (params (TouchedComponent :type "PrimitiveComponent Object Reference") (ButtonPressed :type "Key Structure"))
  ; Robot Right Arm Logic
  ;; Right Arm Clicked, Start Drag
  (set `self.IsDraggingLimb` true :!label _label_5)
  (`self.LoopRightArmDrag`))

(event `UnpauseGame`
  (bind _returnvalue (`GameplayStatics.GetPlayerController` 0))
  (bind _returnvalue_2 (`GameplayStatics.GetPlayerController` 0))
  (bind _demouiwidget (`self.DemoUIWidget`))
  ; Action Inputs
  ;; Unpause Game
  (`GameplayStatics.SetGamePaused` false)
  (set `PlayerController.bEnableClickEvents` true _returnvalue_2)
  (set `PlayerController.bEnableMouseOverEvents` true _returnvalue_2)
  (`Widget.RemoveFromParent` (`self.PauseMenuUIWidget`))
  (`UserWidget.AddToViewport` _demouiwidget 0)
  (`EnhancedInputLibrary.FlushPlayerInput` _returnvalue)
  (`WidgetBlueprintLibrary.SetInputMode_GameAndUIEx` _returnvalue _demouiwidget "DoNotLock" false)
  (`KismetSystemLibrary.Delay` 0.26)
  (set `self.IsMenuOpen` false))

(event `self.RightLowerArmOBJ.OnClicked`
  (params (TouchedComponent :type "PrimitiveComponent Object Reference") (ButtonPressed :type "Key Structure"))
  ; Robot Right Arm Logic
  ;; Right Arm Clicked, Start Drag
  (goto _label_5))

(event `self.RightHandOBJ.OnClicked`
  (params (TouchedComponent :type "PrimitiveComponent Object Reference") (ButtonPressed :type "Key Structure"))
  ; Robot Right Arm Logic
  ;; Right Arm Clicked, Start Drag
  (goto _label_5))

(event `CameraRightRetrigger`
  (bind _returnvalue (`GameplayStatics.GetPlayerController` 0))
  ; Camera Inputs
  ;; Move Camera Right
  (if (not (`self.IsMenuOpen`))
    (`/Engine/EditorBlueprintResources/StandardMacros.Gate` true :!label _label_6
      (:`Exit`
        (`KismetSystemLibrary.K2_SetTimerDelegate` (delegate `CameraRightRetrigger`) 0.025 :!label _label_7)
        (if (`KismetMathLibrary.BooleanNOR` (`PlayerController.IsInputKeyDown` _returnvalue "A") (`PlayerController.IsInputKeyDown` _returnvalue "Left"))
          (`SceneComponent.K2_AddLocalRotation` (`self.OrbitPoint`) (struct :`Yaw` -2.5) false false))))))

(event `InputAction|Reset`
  (params (Key :type "Key Structure"))
  ; Action Inputs
  ;; Reset
  (:`Pressed`
    (`EnhancedInputLibrary.FlushPlayerInput` (`GameplayStatics.GetPlayerController` 0))
    (`SceneComponent.K2_SetRelativeRotation` (`self.OrbitPoint`) (struct :`Yaw` -123.0) false false)
    (set `SpringArmComponent.TargetArmLength` 1000.0 (`self.SpringArm`))
    (`SceneComponent.K2_SetRelativeLocation` (`self.Robot`) (0.0 0.0 0.0) false false)
    (`SceneComponent.K2_SetRelativeLocation` (`self.RightArm`) (0.0 0.0 0.0) false false)
    (`/Game/UI/DemoUI.PrintStatusATTACHED` (`self.DemoUIWidget`))
    (`SceneComponent.K2_AttachToComponent` (`self.RightArm`) (`self.Robot`) "None" "KeepWorld" "KeepWorld" "KeepWorld" true)))

(event `self.TorsoOBJ.OnEndCursorOver`
  (params (TouchedComponent :type "PrimitiveComponent Object Reference"))
  ; Robot Torso Logic
  ;; End Cursor Over, Set Robot Default
  (if (not (`self.IsDraggingLimb`))
    (`PrimitiveComponent.SetMaterial` (`self.TorsoOBJ`) 0 "/Game/Materials/RobotToy/RobotToyMaterial.RobotToyMaterial")
    (`PrimitiveComponent.SetMaterial` (`self.HipsOBJ`) 0 "/Game/Materials/RobotToy/RobotToyMaterial.RobotToyMaterial")
    (`PrimitiveComponent.SetMaterial` (`self.HeadOBJ`) 0 "/Game/Materials/RobotToy/RobotToyMaterial.RobotToyMaterial")
    (`PrimitiveComponent.SetMaterial` (`self.JawOBJ`) 0 "/Game/Materials/RobotToy/RobotToyMaterial.RobotToyMaterial")
    (`PrimitiveComponent.SetMaterial` (`self.LeftEyeOBJ`) 0 "/Game/Materials/RobotToy/RobotToyMaterial.RobotToyMaterial")
    (`PrimitiveComponent.SetMaterial` (`self.RightEyeOBJ`) 0 "/Game/Materials/RobotToy/RobotToyMaterial.RobotToyMaterial")
    (`PrimitiveComponent.SetMaterial` (`self.NeckOBJ`) 0 "/Game/Materials/RobotToy/RobotToyMaterial.RobotToyMaterial")
    (`PrimitiveComponent.SetMaterial` (`self.RightUpperArmOBJ`) 0 "/Game/Materials/RobotToy/RobotToyMaterial.RobotToyMaterial")
    (`PrimitiveComponent.SetMaterial` (`self.RightLowerArmOBJ`) 0 "/Game/Materials/RobotToy/RobotToyMaterial.RobotToyMaterial")
    (`PrimitiveComponent.SetMaterial` (`self.RightHandOBJ`) 0 "/Game/Materials/RobotToy/RobotToyMaterial.RobotToyMaterial")
    (`PrimitiveComponent.SetMaterial` (`self.LeftUpperArmOBJ`) 0 "/Game/Materials/RobotToy/RobotToyMaterial.RobotToyMaterial")
    (`PrimitiveComponent.SetMaterial` (`self.LeftLowerArmOBJ`) 0 "/Game/Materials/RobotToy/RobotToyMaterial.RobotToyMaterial")
    (`PrimitiveComponent.SetMaterial` (`self.LeftHandOBJ`) 0 "/Game/Materials/RobotToy/RobotToyMaterial.RobotToyMaterial")
    (`PrimitiveComponent.SetMaterial` (`self.RightThighOBJ`) 0 "/Game/Materials/RobotToy/RobotToyMaterial.RobotToyMaterial")
    (`PrimitiveComponent.SetMaterial` (`self.RightShinOBJ`) 0 "/Game/Materials/RobotToy/RobotToyMaterial.RobotToyMaterial")
    (`PrimitiveComponent.SetMaterial` (`self.RightFootOBJ`) 0 "/Game/Materials/RobotToy/RobotToyMaterial.RobotToyMaterial")
    (`PrimitiveComponent.SetMaterial` (`self.LeftThighOBJ`) 0 "/Game/Materials/RobotToy/RobotToyMaterial.RobotToyMaterial")
    (`PrimitiveComponent.SetMaterial` (`self.LeftShinOBJ`) 0 "/Game/Materials/RobotToy/RobotToyMaterial.RobotToyMaterial")
    (`PrimitiveComponent.SetMaterial` (`self.LeftFootOBJ`) 0 "/Game/Materials/RobotToy/RobotToyMaterial.RobotToyMaterial")))

(event `self.RightUpperArmOBJ.OnEndCursorOver`
  (params (TouchedComponent :type "PrimitiveComponent Object Reference"))
  ; Robot Right Arm Logic
  ;; Remove Cursor From Right Arm, Set Default Material
  (if (not (`self.IsDraggingLimb`)) :!label _label_8
    (`PrimitiveComponent.SetMaterial` (`self.RightLowerArmOBJ`) 0 "/Game/Materials/RobotToy/RobotToyMaterial.RobotToyMaterial")
    (`PrimitiveComponent.SetMaterial` (`self.RightHandOBJ`) 0 "/Game/Materials/RobotToy/RobotToyMaterial.RobotToyMaterial")
    (`PrimitiveComponent.SetMaterial` (`self.RightUpperArmOBJ`) 0 "/Game/Materials/RobotToy/RobotToyMaterial.RobotToyMaterial")))

(event `self.RightLowerArmOBJ.OnEndCursorOver`
  (params (TouchedComponent :type "PrimitiveComponent Object Reference"))
  ; Robot Right Arm Logic
  ;; Remove Cursor From Right Arm, Set Default Material
  (goto _label_8))

(event `InputAction|CameraRight`
  (params (Key :type "Key Structure"))
  ; Camera Inputs
  ;; Move Camera Right
  (:`Pressed`
    (if (not (`self.IsMenuOpen`))
      (`|ExecutionSequence`
        (:`then_0`
          (goto _label_6 :!via `Open`))
        (:`then_1`
          (goto _label_7)))))
  (:`Released`
    (goto _label_6 :!via `Close`)))

(event `self.RightHandOBJ.OnEndCursorOver`
  (params (TouchedComponent :type "PrimitiveComponent Object Reference"))
  ; Robot Right Arm Logic
  ;; Remove Cursor From Right Arm, Set Default Material
  (goto _label_8))

(event `self.RightUpperArmOBJ.OnBeginCursorOver`
  (params (TouchedComponent :type "PrimitiveComponent Object Reference"))
  ; Robot Right Arm Logic
  ;; Cursor Over Right Arm, Set Right Arm Yellow
  (if (`self.IsDraggingRobot`) :!label _label_9
    _
    (elif (not (`self.IsDraggingLimb`))
      (`PrimitiveComponent.SetMaterial` (`self.RightLowerArmOBJ`) 0 "/Game/Shaders/YellowShader.YellowShader")
      (`PrimitiveComponent.SetMaterial` (`self.RightHandOBJ`) 0 "/Game/Shaders/YellowShader.YellowShader")
      (`PrimitiveComponent.SetMaterial` (`self.RightUpperArmOBJ`) 0 "/Game/Shaders/YellowShader.YellowShader"))))

(event `self.RightLowerArmOBJ.OnBeginCursorOver`
  (params (TouchedComponent :type "PrimitiveComponent Object Reference"))
  ; Robot Right Arm Logic
  ;; Cursor Over Right Arm, Set Right Arm Yellow
  (goto _label_9))

(event `CameraLeftRetrigger`
  (bind _returnvalue (`GameplayStatics.GetPlayerController` 0))
  ; Camera Inputs
  ;; Move Camera Left
  (if (not (`self.IsMenuOpen`))
    (`/Engine/EditorBlueprintResources/StandardMacros.Gate` true :!label _label_10
      (:`Exit`
        (`KismetSystemLibrary.K2_SetTimerDelegate` (delegate `CameraLeftRetrigger`) 0.025 :!label _label_11)
        (if (`KismetMathLibrary.BooleanNOR` (`PlayerController.IsInputKeyDown` _returnvalue "D") (`PlayerController.IsInputKeyDown` _returnvalue "Right"))
          (`SceneComponent.K2_AddLocalRotation` (`self.OrbitPoint`) (struct :`Yaw` 2.5) false false))))))

(event `self.RightHandOBJ.OnBeginCursorOver`
  (params (TouchedComponent :type "PrimitiveComponent Object Reference"))
  ; Robot Right Arm Logic
  ;; Cursor Over Right Arm, Set Right Arm Yellow
  (goto _label_9))

(event `InputAction|CameraLeft`
  (params (Key :type "Key Structure"))
  ; Camera Inputs
  ;; Move Camera Left
  (:`Pressed`
    (if (not (`self.IsMenuOpen`))
      (`|ExecutionSequence`
        (:`then_0`
          (goto _label_10 :!via `Open`))
        (:`then_1`
          (goto _label_11)))))
  (:`Released`
    (goto _label_10 :!via `Close`)))

(event `InputAction|ZoomIn(Mouse)`
  (params (Key :type "Key Structure"))
  (bind _returnvalue (`GameplayStatics.GetPlayerController` 0))
  (bind _springarm (`self.SpringArm`))
  (bind _targetarmlength (`SpringArmComponent.TargetArmLength` _springarm))
  ; Camera Inputs
  ;; Zoom Camera In (Mouse)
  (:`Pressed`
    (if (`self.IsMenuOpen`)
      _
      (elif (`KismetMathLibrary.BooleanNOR` (`PlayerController.IsInputKeyDown` _returnvalue "X") (`PlayerController.IsInputKeyDown` _returnvalue "Z"))
        (if (<= _targetarmlength 400.0)
          (set `SpringArmComponent.TargetArmLength` 300.0 _springarm)
          (else
            (set `SpringArmComponent.TargetArmLength` (- _targetarmlength 100.0) _springarm)))))))

(event `InputAction|ZoomOut(Mouse)`
  (params (Key :type "Key Structure"))
  (bind _returnvalue (`GameplayStatics.GetPlayerController` 0))
  (bind _springarm (`self.SpringArm`))
  (bind _targetarmlength (`SpringArmComponent.TargetArmLength` _springarm))
  ; Camera Inputs
  ;; Zoom Camera Out (Mouse)
  (:`Pressed`
    (if (`self.IsMenuOpen`)
      _
      (elif (`KismetMathLibrary.BooleanNOR` (`PlayerController.IsInputKeyDown` _returnvalue "Z") (`PlayerController.IsInputKeyDown` _returnvalue "X"))
        (if (>= _targetarmlength 5000.0)
          (set `SpringArmComponent.TargetArmLength` 5000.0 _springarm)
          (else
            (set `SpringArmComponent.TargetArmLength` (+ _targetarmlength 100.0) _springarm)))))))

(event `ZoomInRetrigger`
  (bind _returnvalue (`GameplayStatics.GetPlayerController` 0))
  (bind _springarm (`self.SpringArm`))
  (bind _targetarmlength (`SpringArmComponent.TargetArmLength` _springarm))
  ; Camera Inputs
  ;; Zoom Camera In (Keyboard)
  (if (not (`self.IsMenuOpen`))
    (`/Engine/EditorBlueprintResources/StandardMacros.Gate` true :!label _label_12
      (:`Exit`
        (`KismetSystemLibrary.K2_SetTimerDelegate` (delegate `ZoomInRetrigger`) 0.025 :!label _label_13)
        (if (`KismetMathLibrary.BooleanNOR` (`PlayerController.IsInputKeyDown` _returnvalue "X") (`PlayerController.IsInputKeyDown` _returnvalue "MouseWheelAxis"))
          (if (<= _targetarmlength 400.0)
            (set `SpringArmComponent.TargetArmLength` 300.0 _springarm)
            (else
              (set `SpringArmComponent.TargetArmLength` (- _targetarmlength 50.0) _springarm))))))))

(event `InputAction|ZoomIn(Keyboard)`
  (params (Key :type "Key Structure"))
  ; Camera Inputs
  ;; Zoom Camera In (Keyboard)
  (:`Pressed`
    (if (not (`self.IsMenuOpen`))
      (`|ExecutionSequence`
        (:`then_0`
          (goto _label_12 :!via `Open`))
        (:`then_1`
          (goto _label_13)))))
  (:`Released`
    (goto _label_12 :!via `Close`)))

(event `ZoomOutRetrigger`
  (bind _returnvalue (`GameplayStatics.GetPlayerController` 0))
  (bind _springarm (`self.SpringArm`))
  (bind _targetarmlength (`SpringArmComponent.TargetArmLength` _springarm))
  ; Camera Inputs
  ;; Zoom Camera Out (Keyboard)
  (if (not (`self.IsMenuOpen`))
    (`/Engine/EditorBlueprintResources/StandardMacros.Gate` true :!label _label_14
      (:`Exit`
        (`KismetSystemLibrary.K2_SetTimerDelegate` (delegate `ZoomOutRetrigger`) 0.025 :!label _label_15)
        (if (`KismetMathLibrary.BooleanNOR` (`PlayerController.IsInputKeyDown` _returnvalue "Z") (`PlayerController.IsInputKeyDown` _returnvalue "MouseWheelAxis"))
          (if (>= _targetarmlength 5000.0)
            (set `SpringArmComponent.TargetArmLength` 5000.0 _springarm)
            (else
              (set `SpringArmComponent.TargetArmLength` (+ _targetarmlength 50.0) _springarm))))))))

(event `InputAction|ZoomOut(Keyboard)`
  (params (Key :type "Key Structure"))
  ; Camera Inputs
  ;; Zoom Camera Out (Keyboard)
  (:`Pressed`
    (if (not (`self.IsMenuOpen`))
      (`|ExecutionSequence`
        (:`then_0`
          (goto _label_14 :!via `Open`))
        (:`then_1`
          (goto _label_15)))))
  (:`Released`
    (goto _label_14 :!via `Close`)))

(event `InputAction|SnapToAngle1`
  (params (Key :type "Key Structure"))
  ; Camera Inputs
  ;; Snap Camera Angle
  (:`Pressed`
    (if (not (`self.IsMenuOpen`))
      (`SceneComponent.K2_SetRelativeRotation` (`self.OrbitPoint`) (struct :`Yaw` 270.0) false false)
      (`SceneComponent.K2_SetRelativeRotation` :`self` (`self.SpringArm`)))))

(event `InputAction|SnapToAngle3`
  (params (Key :type "Key Structure"))
  ; Camera Inputs
  ;; Snap Camera Angle
  (:`Pressed`
    (if (not (`self.IsMenuOpen`))
      (`SceneComponent.K2_SetRelativeRotation` (`self.OrbitPoint`) (struct :`Yaw` 90.0) false false)
      (`SceneComponent.K2_SetRelativeRotation` :`self` (`self.SpringArm`)))))

(event `InputAction|SnapToAngle2`
  (params (Key :type "Key Structure"))
  ; Camera Inputs
  ;; Snap Camera Angle
  (:`Pressed`
    (if (not (`self.IsMenuOpen`))
      (`SceneComponent.K2_SetRelativeRotation` (`self.OrbitPoint`) (struct :`Yaw` 180.0) false false)
      (`SceneComponent.K2_SetRelativeRotation` :`self` (`self.SpringArm`)))))

(event `InputAction|SnapToAngle4`
  (params (Key :type "Key Structure"))
  ; Camera Inputs
  ;; Snap Camera Angle
  (:`Pressed`
    (if (not (`self.IsMenuOpen`))
      (`SceneComponent.K2_SetRelativeRotation` :`self` (`self.OrbitPoint`))
      (`SceneComponent.K2_SetRelativeRotation` :`self` (`self.SpringArm`)))))

(fn `UserConstructionScript`)